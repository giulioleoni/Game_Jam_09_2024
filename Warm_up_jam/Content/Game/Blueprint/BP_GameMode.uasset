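; Game mode for a potion-mixing game that sets the requested recipe and judges the player's mix.
; RandomPotion copies one of three predefined ingredient lists into WantedPotion, and AddIngredient collects ingredients into CurrentPotion.
; At three ingredients, an order-independent containment check either awards points through the cached BP_GameInstance or calls RandomTransform, clearing WantedPotion either way.
; RandomTransform and CurrentPersonDespawn are empty events, and CurrentPotion is not cleared here.
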(event `self.ReceiveBeginPlay`
  (bind _asbp_game_instance (cast `/Game/Game/Blueprint/BP_GameInstance` (`GameplayStatics.GetGameInstance`)))
  (set `self.As BP Game Instance` _asbp_game_instance))

(event `RandomPotion`
  (switch `int` (`KismetMathLibrary.RandomIntegerInRange` 0 2)
    (:`0`
      (for _array_element (`self.PotionA`)
        (`KismetArrayLibrary.Array_Add` (`self.WantedPotion`) _array_element)))
    (:`1`
      (for _array_element_2 (`self.PotionB`)
        (`KismetArrayLibrary.Array_Add` (`self.WantedPotion`) _array_element_2)))
    (:`2`
      (for _array_element_3 (`self.PotionC`)
        (`KismetArrayLibrary.Array_Add` (`self.WantedPotion`) _array_element_3)))))

(event `RandomTransform`)

(event `CurrentPersonDespawn`)

(fn `AddIngredient`
  (params (Ingredient :type "/Game/Game/Blueprint/E_IngredientTypes Enum" :default "NewEnumerator0"))
  (bind _currentpotion (`self.CurrentPotion`))
  (`KismetArrayLibrary.Array_Add` _currentpotion Ingredient)
  (if (== (`KismetArrayLibrary.Array_Length` _currentpotion) 3)
    (for _array_element (`self.WantedPotion`)
      (if (not (`KismetArrayLibrary.Array_Contains` (`self.CurrentPotion`) _array_element))
        (`self.RandomTransform`)
        (`KismetArrayLibrary.Array_Clear` (`self.WantedPotion`))
        (return)))
    (`KismetArrayLibrary.Array_Clear` (`self.WantedPotion`))
    (`/Game/Game/Blueprint/BP_GameInstance.AddPoints` (`self.As BP Game Instance`))))

(fn `UserConstructionScript`)